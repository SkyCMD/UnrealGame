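; Player character Blueprint that adds dash effects, crate smashing, camera zoom triggers, sounds and death/respawn handling.
; Tick watches the dash flags, set outside these graphs, to spawn a charge circle and a one-shot shockwave using latch booleans.
; Capsule overlaps break crates while dashing and restore the dash, or copy zoom settings from BP_ZoomScript actors.
; Killem fades out and disables input, while Respawn returns to StartPos and restores both.
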(event `self.ReceiveBeginPlay`
  (set `self.SpawnedDashEmitter` false)
  (`GameplayStatics.PlaySound2D` "/Game/StarterContent/Audio/Starter_Music01.Starter_Music01" 0.8 1.0 0.0 null null))

(event `self.OnJumped`
  (`GameplayStatics.PlaySoundAtLocation` "/Game/OurContent/Audio/JumpGrunt.JumpGrunt" (`self.K2_GetActorLocation`) (struct) 1.0 0.85 0.0 null null null))

(event `self.ReceiveTick`
  (params (DeltaSeconds :type "Float (single-precision)"))
  (bind _returnvalue (`SceneComponent.K2_GetComponentLocation` (`Actor.RootComponent` (`GameplayStatics.GetPlayerCharacter` 0))))
  (if (`self.prepForDash`)
    (if (not (`self.SpawnedDashEmitter`))
      (bind _returnvalue_2 (`GameplayStatics.SpawnEmitterAtLocation` "/Game/FXVarietyPack/Particles/P_ky_magicCircle1.P_ky_magicCircle1" (`KismetMathLibrary.MakeVector` (.x _returnvalue) (.y _returnvalue) (- (.z _returnvalue) 85.0))))
      (set `self.SpawnedDashEmitter` true))
    (elif (`self.dashing`)
      (if (not (`self.SpawnedDashImpact`))
        (`GameplayStatics.SpawnEmitterAtLocation` "/Game/FXVarietyPack/Particles/P_ky_shotShockwave.P_ky_shotShockwave" _returnvalue (struct) (2.0 2.0 2.0))
        (set `self.SpawnedDashEmitter` false)
        (set `self.SpawnedDashImpact` true)
        (`GameplayStatics.PlaySound2D` "/Game/StarterContent/Audio/Explosion02.Explosion02" 1.0 1.0 0.0 null null)
        (`KismetSystemLibrary.Delay` 0.25)
        (`ActorComponent.Deactivate` _returnvalue_2))
      (else
        (set `self.SpawnedDashImpact` false)))))

(event `self.CapsuleComponent.OnComponentBeginOverlap`
  (params (OverlappedComponent :type "PrimitiveComponent Object Reference") (OtherActor :type "Actor Object Reference") (OtherComp :type "PrimitiveComponent Object Reference") (OtherBodyIndex :type Integer) (bFromSweep :type Boolean) (SweepResult :type "HitResult Structure (by ref)"))
  (bind _returnvalue (`SceneComponent.K2_GetComponentLocation` (`Actor.RootComponent` (`GameplayStatics.GetPlayerCharacter` 0))))
  (bind _asbp_crate (cast `/Game/OurContent/Blueprints/BP_Crate` OtherActor)
    (:`then`
      (if (`self.dashing`)
        (if (not (`BreakableCrate.broken` _asbp_crate))
          (set `self.CanDash` true)
          (`GameplayStatics.SpawnEmitterAtLocation` "/Game/InfinityBladeEffects/Effects/FX_Breakables/Box/P_BoxBreak_Wood_Lrg_01.P_BoxBreak_Wood_Lrg_01" (`self.K2_GetActorLocation` _asbp_crate) (struct) (2.0 2.0 2.0))
          (set `BreakableCrate.broken` true _asbp_crate)
          (set `self.HitBox` true)
          (`SceneComponent.SetVisibility` (`BreakableCrate.BoxMesh` _asbp_crate) false false)
          (`GameplayStatics.SpawnEmitterAtLocation` "/Game/FXVarietyPack/Particles/P_ky_hit2.P_ky_hit2" _returnvalue (struct) (2.0 2.0 2.0))
          (`self.K2_DestroyActor` _asbp_crate)
          (`GameplayStatics.PlaySoundAtLocation` "/Game/OurContent/Audio/BreakingCrate.BreakingCrate" _returnvalue (struct) 1.0 1.0 0.0 null null null))))
    (:`CastFailed`
      (bind _asbp_zoom_script (cast `/Game/OurContent/Blueprints/BP_ZoomScript` OtherActor))
      (set `self.zoomLevel` (`/Game/OurContent/Blueprints/BP_ZoomScript.ZoomValue` _asbp_zoom_script))
      (set `self.zoomSpeed` (`/Game/OurContent/Blueprints/BP_ZoomScript.ZoomSpeed` _asbp_zoom_script)))))

(event `self.OnLanded`
  (params (Hit :type "HitResult Structure (by ref)"))
  (set `self.CanDash` true))

(fn `Killem`
  (bind _asmain_player (cast `MainPlayer` (`GameplayStatics.GetPlayerCharacter` 0)))
  (`PlayerCameraManager.StartCameraFade` :`self` (`GameplayStatics.GetPlayerCameraManager` 0) :`ToAlpha` 1.0 :`Duration` 0.75)
  (`self.DisableInput` _asmain_player (`GameplayStatics.GetPlayerController` 0)))

(fn `Respawn`
  (`self.K2_SetActorLocation` (`self.startPos`))
  (`PlayerCameraManager.StartCameraFade` :`self` (`GameplayStatics.GetPlayerCameraManager` 0) :`FromAlpha` 1.0 :`Duration` 0.5)
  (`self.EnableInput` null))

(fn `UserConstructionScript`)