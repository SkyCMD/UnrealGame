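; BP_Train is a train actor that plays its sound once triggered by the player and explodes on reaching its end.
; Overlap of CollisionBox by MainPlayer sets StartMoving, and Tick then spawns the train audio once.
; When ReachedEnd is true, Tick stops that audio and spawns a one-time explosion with sound and a persistent fire, both offset along world Y.
; Movement and the setting of ReachedEnd are absent from these graphs.
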(event `self.ReceiveTick`
  (params (DeltaSeconds :type "Float (single-precision)"))
  (bind _returnvalue (`self.K2_GetActorLocation`))
  (if (and (`self.startMoving`) (not (`self.PlayedStartSound`)))
    (bind _returnvalue_2 (`GameplayStatics.SpawnSoundAtLocation` "/Game/OurContent/Audio/train.train" _returnvalue (struct) 0.3 1.0 0.0 null null))
    (set `self.TrainSound` _returnvalue_2)
    (set `self.PlayedStartSound` true)
    (elif (and (`self.reachedEnd`) (not (`self.Exploded`)))
      (`GameplayStatics.SpawnEmitterAtLocation` "/Game/Built_In_Content/StarterContent/Particles/P_Explosion.P_Explosion" (`KismetMathLibrary.MakeVector` (.x _returnvalue) (- (.y _returnvalue) 2500.0) (.z _returnvalue)) (struct) (40.0 40.0 40.0))
      (`GameplayStatics.PlaySoundAtLocation` "/Game/StarterContent/Audio/Explosion01.Explosion01" _returnvalue (struct) 2.0 0.9 0.0 null null null)
      (set `self.Exploded` true)
      (`AudioComponent.Stop` (`self.TrainSound`))
      (`GameplayStatics.SpawnEmitterAtLocation` "/Game/StarterContent/Particles/P_Fire.P_Fire" (`KismetMathLibrary.MakeVector` (.x _returnvalue) (- (.y _returnvalue) 3000.0) (.z _returnvalue)) (struct :`Roll` 20.0) (20.0 20.0 20.0) false))))

(event `self.CollisionBox.OnActorBeginOverlap`
  (params (OverlappedActor :type "Actor Object Reference") (OtherActor :type "Actor Object Reference"))
  (cast `MainPlayer` OtherActor)
  (set `self.startMoving` true))

(fn `UserConstructionScript`)