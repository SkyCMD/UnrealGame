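; BP_Character is a character Blueprint that drives the visual effects for a dash move.
; Tick watches the PrepForDash and Dashing flags, with spawn guards so each effect plays once.
; Dash prep spawns a magic circle near player 0's feet.
; Dashing spawns a scaled shockwave at the player, then deactivates the circle after a short delay.
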(event `self.ReceiveBeginPlay`
  (set `self.SpawnedDashEmitter` false)
  (set `self.DelayTime` 2.0))

(event `self.ReceiveTick`
  (params (DeltaSeconds :type "Float (single-precision)"))
  (bind _returnvalue (`SceneComponent.K2_GetComponentLocation` (`Actor.RootComponent` (`GameplayStatics.GetPlayerCharacter` 0))))
  (if (`self.prepForDash`)
    (if (not (`self.SpawnedDashEmitter`))
      (bind _returnvalue_2 (`GameplayStatics.SpawnEmitterAtLocation` "/Game/FXVarietyPack/Particles/P_ky_magicCircle1.P_ky_magicCircle1" (`KismetMathLibrary.MakeVector` (.x _returnvalue) (.y _returnvalue) (- (.z _returnvalue) 85.0))))
      (set `self.SpawnedDashEmitter` true))
    (elif (`self.dashing`)
      (if (not (`self.SpawnedDashImpact`))
        (`GameplayStatics.SpawnEmitterAtLocation` "/Game/FXVarietyPack/Particles/P_ky_shotShockwave.P_ky_shotShockwave" _returnvalue (struct) (2.0 2.0 2.0))
        (set `self.SpawnedDashEmitter` false)
        (set `self.SpawnedDashImpact` true)
        (`KismetSystemLibrary.Delay` 0.25)
        (`ActorComponent.Deactivate` _returnvalue_2))
      (else
        (set `self.SpawnedDashImpact` false)))))

(fn `UserConstructionScript`)